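; BP_HealthPickup is a collectible that restores health to the third-person player character.
; When that character overlaps its box, it adds a fixed health amount, unless health is already at the cap.
; It plays a sound and a brief spark burst, then after a short delay stops the particles, updates the HUD through UpdateLives and destroys itself.
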(event OnComponentBeginOverlap(Box)
  (params (OverlappedComponent :type Primitive%20Component%20Object%20Reference) (OtherActor :type Actor%20Object%20Reference) (OtherComp :type Primitive%20Component%20Object%20Reference) (OtherBodyIndex :type Integer) (bFromSweep :type Boolean) (SweepResult :type Hit%20Result%20Structure%20%28by%20ref%29))
  (bind _returnvalue (Transformation|GetActorLocation))
  (bind _asbp_third_person_character (Utilities|Casting|CastToBP_ThirdPersonCharacter OtherActor))
  (if (not (>= (Variables|/Game/ThirdPerson/Blueprints/BP_ThirdPersonCharacter.BP_ThirdPersonCharacter_C|GetHealth _asbp_third_person_character) 1000))
    (bind _output_get (Variables|/Game/ThirdPerson/Blueprints/BP_ThirdPersonCharacter.BP_ThirdPersonCharacter_C|SetHealth _asbp_third_person_character (+ (Variables|/Game/ThirdPerson/Blueprints/BP_ThirdPersonCharacter.BP_ThirdPersonCharacter_C|GetHealth _asbp_third_person_character) 100)))
    (Audio|PlaySoundatLocation "/Game/Sounds/Health.Health" _returnvalue "0, 0, 0" 1.0 1.0 0.0 0 0 0 0)
    (bind _returnvalue_2 (Effects|SpawnEmitteratLocation "/Game/StarterContent/Particles/sparks2.sparks2" _returnvalue "0, 0, 0" "50.000000,50.000000,50.000000"))
    (Utilities|FlowControl|Delay 0.25)
    (Components|Activation|Deactivate _returnvalue_2)
    (Default|UpdateLives (Variables|/Game/ThirdPerson/Blueprints/BP_ThirdPersonCharacter.BP_ThirdPersonCharacter_C|GetHUD _asbp_third_person_character) _output_get)
    (Actor|DestroyActor)))

(event EventBeginPlay)

(event Collision|EventActorBeginOverlap
  (params (OtherActor :type Actor%20Object%20Reference)))

(event EventTick
  (params (DeltaSeconds :type Float%20%28single-precision%29)))

(fn ConstructionScript)