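; BP_EndLevelFlag is an end-of-level flag that completes the level when the player overlaps its Box with enough Score.
; A Score of at least a hardcoded five shows the HUD's Levelcomplete element, pauses the game and switches to UI-only input with a cursor; otherwise a message prints.
; BeginPlay caches the player character and counts BP_Parts actors into PartsRequired, which the check never uses.
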(event OnComponentBeginOverlap(Box)
  (params (OverlappedComponent :type Primitive%20Component%20Object%20Reference) (OtherActor :type Actor%20Object%20Reference) (OtherComp :type Primitive%20Component%20Object%20Reference) (OtherBodyIndex :type Integer) (bFromSweep :type Boolean) (SweepResult :type Hit%20Result%20Structure%20%28by%20ref%29))
  (bind _returnvalue (Game|GetPlayerController 0))
  (bind _asbp_third_person_character (Utilities|Casting|CastToBP_ThirdPersonCharacter OtherActor))
  (if (>= (Variables|/Game/ThirdPerson/Blueprints/BP_ThirdPersonCharacter.BP_ThirdPersonCharacter_C|GetScore _asbp_third_person_character) 5)
    (Widget|SetVisibility (Variables|/Game/UI/WB_RobotHud.WB_RobotHud_C|GetLevelcomplete (Variables|/Game/ThirdPerson/Blueprints/BP_ThirdPersonCharacter.BP_ThirdPersonCharacter_C|GetHUD (Variables|Default|GetAs%20BP%20Third%20Person%20Character))) "Visible")
    (Game|SetGamePaused true)
    (Variables|/Script/Engine.PlayerController|SetbShowMouseCursor _returnvalue true)
    (Input|SetInputModeUIOnly _returnvalue 0 "DoNotLock" false)
    (else
      (Development|PrintString "you require more parts to proceed"))))

(event EventBeginPlay
  (bind _outactors (Actor|GetAllActorsOfClass "/Game/Collectibles/BP_Parts.BP_Parts_C"))
  (Variables|Default|SetPartsRequired (Utilities|Array|Length _outactors))
  (bind _asbp_third_person_character (Utilities|Casting|CastToBP_ThirdPersonCharacter (Game|GetPlayerCharacter 0)))
  (Variables|Default|SetAs%20BP%20Third%20Person%20Character _asbp_third_person_character))

(event Collision|EventActorBeginOverlap
  (params (OtherActor :type Actor%20Object%20Reference)))

(event EventTick
  (params (DeltaSeconds :type Float%20%28single-precision%29)))

(fn ConstructionScript)