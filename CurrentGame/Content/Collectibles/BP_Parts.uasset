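; BP_Parts is a collectible part that the player picks up by walking into its box trigger.
; On overlap it increments the third-person character's Score and passes the new count to that character's HUD parts display.
; It plays a sound and a sparks emitter at its location, then after a short delay deactivates the emitter and destroys itself.
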(event OnComponentBeginOverlap(Box)
  (params (OverlappedComponent :type Primitive%20Component%20Object%20Reference) (OtherActor :type Actor%20Object%20Reference) (OtherComp :type Primitive%20Component%20Object%20Reference) (OtherBodyIndex :type Integer) (bFromSweep :type Boolean) (SweepResult :type Hit%20Result%20Structure%20%28by%20ref%29))
  (bind _asbp_third_person_character (Utilities|Casting|CastToBP_ThirdPersonCharacter OtherActor))
  (bind _result (Math|Integer|IncrementInt (Variables|/Game/ThirdPerson/Blueprints/BP_ThirdPersonCharacter.BP_ThirdPersonCharacter_C|GetScore _asbp_third_person_character))
    (:%20%20
      (Default|UpdateParts (Variables|/Game/ThirdPerson/Blueprints/BP_ThirdPersonCharacter.BP_ThirdPersonCharacter_C|GetHUD _asbp_third_person_character) _result)
      (Audio|PlaySoundatLocation "/Game/Sounds/Tool.Tool" (Transformation|GetActorLocation) "0, 0, 0" 1.0 1.0 0.0 0 0 0 0)
      (bind _returnvalue (Effects|SpawnEmitteratLocation "/Game/StarterContent/Particles/P_Sparks.P_Sparks" (Transformation|GetActorLocation) "0, 0, 0" "50.000000,50.000000,50.000000"))
      (Utilities|FlowControl|Delay 0.25)
      (Components|Activation|Deactivate _returnvalue)
      (Actor|DestroyActor))))

(fn ConstructionScript)