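; Enemy character that chases the player once seen, plays an attack montage on arrival and damages the player on capsule overlap.
; PawnSensing starts an AIMoveTo; a CanAttack flag and DoOnce, reset after the montage plus a short delay, gate the attack.
; Tick halts movement until the player is seen, and the seen flag effectively never clears.
; TakeDamages removes one health per call and destroys the enemy at zero.
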(event OnSeePawn(PawnSensing)
  (params (Pawn :type Pawn%20Object%20Reference))
  (Variables|Default|SetIsSeeingPlayer true)
  (CallFunction|FollowPlayer))

(event OnComponentBeginOverlap(CapsuleComponent)
  (params (OverlappedComponent :type Primitive%20Component%20Object%20Reference) (OtherActor :type Actor%20Object%20Reference) (OtherComp :type Primitive%20Component%20Object%20Reference) (OtherBodyIndex :type Integer) (bFromSweep :type Boolean) (SweepResult :type Hit%20Result%20Structure%20%28by%20ref%29))
  (bind _asbp_third_person_character (Utilities|Casting|CastToBP_ThirdPersonCharacter OtherActor))
  (Default|TakeDamage _asbp_third_person_character (Variables|Default|GetDamageAmounts)))

(event Custom|FollowPlayer
  (Variables|Default|SetCanAttack true)
  (if (Variables|Default|GetIsSeeingPlayer)
    (AI|AIMoveTo self "0, 0, 0" (Game|GetPlayerCharacter 0) 2e+01 false
      (:OnSuccess
        (if (Variables|Default|GetCanAttack)
          (Variables|Default|SetCanAttack false)
          (Utilities|FlowControl|DoOnce false :!label _label
            (:Completed
              (bind _returnvalue (Animation|PlayAnimMontage "/Game/Characters/Mannequins/Anims/Unarmed/Attack/MM_Attack_01_Montage.MM_Attack_01_Montage" 1.0 "None"))
              (Utilities|FlowControl|Delay (+ _returnvalue 0.5))
              (goto _label Reset))))))
    (else
      (Variables|Default|SetIsSeeingPlayer false))))

(event EventBeginPlay)

(event Collision|EventActorBeginOverlap
  (params (OtherActor :type Actor%20Object%20Reference)))

(event EventTick
  (params (DeltaSeconds :type Float%20%28single-precision%29))
  (if (not (Variables|Default|GetIsSeeingPlayer))
    (Components|Movement|StopMovementImmediately (Variables|Character|GetCharacterMovement))))

(fn ConstructionScript)

(fn TakeDamages
  (bind _output_get (Variables|Default|SetEnemyHealth (- (Variables|Default|GetEnemyHealth) 1.0)))
  (if (<= _output_get 0.0)
    (Actor|DestroyActor)))